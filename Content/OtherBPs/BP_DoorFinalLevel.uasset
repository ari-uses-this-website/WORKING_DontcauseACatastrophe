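; BP_DoorFinalLevel is the exit door of the final level, which wins the game once the player has gathered everything.
; On BeginPlay it counts all BP_Fish and BP_RatLINE actors in the level to set the required totals.
; When BP_PaperCatCharacte enters its box with matching Fish and RatMeter values, it shows the won screen, pauses, switches to UI-only input with cursor and plays the victory jingle.
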(event `self.ReceiveBeginPlay`
  (`|ExecutionSequence`
    (:`then_0`
      (bind _outactors (`GameplayStatics.GetAllActorsOfClass` "/Game/OtherBPs/BP_Fish.BP_Fish_C"))
      (set `self.Fishrequired` (`KismetArrayLibrary.Array_Length` _outactors)))
    (:`then_1`
      (bind _outactors_2 (`GameplayStatics.GetAllActorsOfClass` "/Game/Enemies/BP_RatLINE.BP_RatLINE_C"))
      (set `self.rats required` (`KismetArrayLibrary.Array_Length` _outactors_2)))))

(event `self.Box.OnComponentBeginOverlap`
  (params (OverlappedComponent :type "PrimitiveComponent Object Reference") (OtherActor :type "Actor Object Reference") (OtherComp :type "PrimitiveComponent Object Reference") (OtherBodyIndex :type Integer) (bFromSweep :type Boolean) (SweepResult :type "HitResult Structure (by ref)"))
  (bind _returnvalue (`GameplayStatics.GetPlayerController` 0))
  (bind _asbp_paper_cat_characte (cast `/Game/PaperCatCharacter/BP_PaperCatCharacte` OtherActor))
  (if (and (== (`/Game/PaperCatCharacter/BP_PaperCatCharacte.Fish` _asbp_paper_cat_characte) (`self.Fishrequired`)) (== (`/Game/PaperCatCharacter/BP_PaperCatCharacte.Rat Meter` _asbp_paper_cat_characte) (`self.rats required`)))
    (`Widget.SetVisibility` (`/Game/UI/WB_Timer.GameWOn` (`/Game/PaperCatCharacter/BP_PaperCatCharacte.PlayerHUD ref` _asbp_paper_cat_characte)) "Visible")
    (`GameplayStatics.SetGamePaused` true)
    (set `PlayerController.bShowMouseCursor` true _returnvalue)
    (`WidgetBlueprintLibrary.SetInputMode_UIOnlyEx` _returnvalue null)
    (`GameplayStatics.PlaySound2D` "/Game/Sounds/Music/Level_Won_Jingle.Level_Won_Jingle" 1.0 1.0 0.0 null null)))

(fn `UserConstructionScript`)