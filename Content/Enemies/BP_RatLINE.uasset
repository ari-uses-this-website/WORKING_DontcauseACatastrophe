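; Paper-sprite rat enemy that walks forward constantly and turns around when a short line trace hits an actor tagged BLOK.
; A second gated trace damages the player cat by the rat's clamped Health, toggling the gate around a short delay as a cooldown.
; UpdateHealth subtracts damage and calls Dead, which at exactly zero health increments the player's RatMeter, updates the HUD, plays death effects and destroys the rat.
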(event `self.CapsuleComponent.OnComponentHit`
  (params (HitComponent :type "PrimitiveComponent Object Reference") (OtherActor :type "Actor Object Reference") (OtherComp :type "PrimitiveComponent Object Reference") (NormalImpulse :type "Vector Structure") (Hit :type "HitResult Structure (by ref)")))

(event `self.ReceiveBeginPlay`
  (bind _asbp_paper_cat_characte (cast `/Game/PaperCatCharacter/BP_PaperCatCharacte` (`GameplayStatics.GetPlayerCharacter` 0)))
  (set `self.As BP Paper Cat Characte` _asbp_paper_cat_characte))

(event `self.ReceiveTick`
  (params (DeltaSeconds :type "Float (single-precision)"))
  (bind _sprite (`self.Sprite`))
  (bind _sprite_2 (`self.Sprite`))
  (bind _returnvalue (`SceneComponent.K2_GetComponentLocation` _sprite))
  (bind _returnvalue_2 (`SceneComponent.K2_GetComponentLocation` _sprite_2))
  ; Line Trace for turning around when sensing something with the BLOK tag
  (`|ExecutionSequence`
    (:`then_0`
      (`self.AddMovementInput` (`self.GetActorForwardVector`))
      (bind _outhit (`KismetSystemLibrary.LineTraceSingle` _returnvalue (+ _returnvalue (* (`SceneComponent.GetForwardVector` _sprite) 20)) "TraceTypeQuery1"))
      (if (`GameplayStatics.BreakHitResult` _outhit)
        (if (`self.ActorHasTag` (`.HitActor` (`GameplayStatics.BreakHitResult` _outhit)) "BLOK")
          (`self.TurnAround`))))
    (:`then_1`
      (`/Engine/EditorBlueprintResources/StandardMacros.Gate` false :!label _label
        (:`Exit`
          (bind _outhit_2 (`KismetSystemLibrary.LineTraceSingle` :`Start` _returnvalue_2 :`End` (+ _returnvalue_2 (* (`SceneComponent.GetForwardVector` _sprite_2) 25)) :`TraceChannel` "TraceTypeQuery1" :`DrawDebugType` "ForDuration"))
          (bind _asbp_paper_cat_characte (cast `/Game/PaperCatCharacter/BP_PaperCatCharacte` (`.HitActor` (`GameplayStatics.BreakHitResult` _outhit_2))))
          (`self.Toogle damage`)
          (`/Game/PaperCatCharacter/BP_PaperCatCharacte.Take Damage` _asbp_paper_cat_characte (`KismetMathLibrary.Clamp` (`self.Health`) 0 50))
          (`KismetSystemLibrary.Delay` 0.5)
          (`self.Toogle damage`))))))

(event `Toogle damage`
  (goto _label :!via `Toggle`))

(fn `Dead`
  (bind _as_bp_paper_cat_characte (`self.As BP Paper Cat Characte`))
  (bind _output_get (set `self.IsDead` (== (`self.Health`) 0)))
  (if _output_get
    (bind _result (`/Engine/EditorBlueprintResources/StandardMacros.IncrementInt` (`/Game/PaperCatCharacter/BP_PaperCatCharacte.Rat Meter` _as_bp_paper_cat_characte))
      (:`  `
        (`/Engine/EditorBlueprintResources/StandardMacros.IsValid` _as_bp_paper_cat_characte
          (:`Is Valid`
            (`/Game/UI/WB_Timer.Update Rats` (`/Game/PaperCatCharacter/BP_PaperCatCharacte.PlayerHUD ref` _as_bp_paper_cat_characte) _result)
            (`NiagaraFunctionLibrary.SpawnSystemAtLocation` "/Game/FX/RatFX/NE_RatDead_System3.NE_RatDead_System3" (`SceneComponent.K2_GetComponentLocation` (`self.Sprite`)))
            (`GameplayStatics.PlaySound2D` "/Game/Sounds/DeathBell.DeathBell" 1.0 1.0 0.0 null null)
            (`self.K2_DestroyActor`)))))))

(fn `TurnAround`
  (`self.K2_SetActorRotation` (`KismetMathLibrary.ComposeRotators` (`self.K2_GetActorRotation`) (struct :`Yaw` 180.0))))

(fn `Turnaroundobstacle`
  (`self.K2_SetActorRotation` (`KismetMathLibrary.ComposeRotators` (`self.K2_GetActorRotation`) (struct :`Yaw` 180.0))))

(fn `UpdateHealth`
  (params (Damage :type Integer))
  (bind _output_get (set `self.Health` (- (`self.Health`) Damage)))
  (if (<= _output_get 0)
    (`self.Dead`)))

(fn `UserConstructionScript`)