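; BP_RatOLD is a rat enemy that walks constantly along its forward vector and turns around when its wall detection overlaps something.
; Overlapping the paper cat player deals damage to the cat, takes some of the rat's own health and also flips its direction.
; When its health hits exactly zero, it increments the cat's RatMeter, updates the rat count on the player HUD and destroys itself.
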(event `self.ReceiveBeginPlay`
  (bind _asbp_paper_cat_characte (cast `/Game/PaperCatCharacter/BP_PaperCatCharacte` (`GameplayStatics.GetPlayerCharacter` 0)))
  (set `self.As BP Paper Cat Characte` _asbp_paper_cat_characte))

(event `self.ReceiveTick`
  (params (DeltaSeconds :type "Float (single-precision)"))
  (`self.AddMovementInput` (`self.GetActorForwardVector`)))

(event `self.PlayerDetection.OnComponentBeginOverlap`
  (params (OverlappedComponent :type "PrimitiveComponent Object Reference") (OtherActor :type "Actor Object Reference") (OtherComp :type "PrimitiveComponent Object Reference") (OtherBodyIndex :type Integer) (bFromSweep :type Boolean) (SweepResult :type "HitResult Structure (by ref)"))
  (bind _asbp_paper_cat_characte (cast `/Game/PaperCatCharacter/BP_PaperCatCharacte` OtherActor))
  (`/Game/PaperCatCharacter/BP_PaperCatCharacte.Take Damage` _asbp_paper_cat_characte 100)
  (`self.UpdateHealth` 10)
  (`self.TurnAround`))

(event `self.WallDetection.OnComponentBeginOverlap`
  (params (OverlappedComponent :type "PrimitiveComponent Object Reference") (OtherActor :type "Actor Object Reference") (OtherComp :type "PrimitiveComponent Object Reference") (OtherBodyIndex :type Integer) (bFromSweep :type Boolean) (SweepResult :type "HitResult Structure (by ref)"))
  (`self.Turnaroundobstacle`))

(fn `Dead`
  (bind _as_bp_paper_cat_characte (`self.As BP Paper Cat Characte`))
  (bind _output_get (set `self.IsDead` (== (`self.Health`) 0)))
  (if _output_get
    (bind _result (`/Engine/EditorBlueprintResources/StandardMacros.IncrementInt` (`/Game/PaperCatCharacter/BP_PaperCatCharacte.Rat Meter` _as_bp_paper_cat_characte))
      (:`  `
        (`/Engine/EditorBlueprintResources/StandardMacros.IsValid` _as_bp_paper_cat_characte
          (:`Is Valid`
            (`/Game/UI/WB_Timer.Update Rats` (`/Game/PaperCatCharacter/BP_PaperCatCharacte.PlayerHUD ref` _as_bp_paper_cat_characte) _result)
            (`self.K2_DestroyActor`)))))))

(fn `TurnAround`
  (`self.K2_SetActorRotation` (`KismetMathLibrary.ComposeRotators` (`self.K2_GetActorRotation`) (struct :`Yaw` 180.0))))

(fn `Turnaroundobstacle`
  (`self.K2_SetActorRotation` (`KismetMathLibrary.ComposeRotators` (`self.K2_GetActorRotation`) (struct :`Yaw` 180.0))))

(fn `UpdateHealth`
  (params (Damage :type Integer))
  (bind _output_get (set `self.Health` (- (`self.Health`) Damage)))
  (if (<= _output_get 0)
    (`self.Dead`)))

(fn `UserConstructionScript`)